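; Rhythm-timed panel that dashes the player to a linked NextPanel when Dash or Teleport is pressed while standing on it.
; An on-beat press adds combo and disables movement while Tick lerps the character over half a beat, with a trail.
; A mistimed press disables the panel's collision for one second.
; An arrow cylinder aligns toward NextPanel and alternates materials on BeatFunction, turning black without a link.
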(event Collision|EventActorBeginOverlap
  (params (OtherActor :type Actor%20Object%20Reference))
  (if (== (Utilities|GetClass OtherActor) "/Game/BP/Player/ThirdPersonCharacter.ThirdPersonCharacter_C")
    (Variables|Default|SetRide true)))

(event EventTick
  (params (DeltaSeconds :type Float%20%28single-precision%29))
  (bind _beginvec (Variables|Default|Getbeginvec))
  (bind _nextpanel (Variables|Default|GetNextPanel))
  (bind _returnvalue (Transformation|GetActorLocation _nextpanel))
  (bind _returnvalue_2 (- _returnvalue _beginvec))
  (bind (_x _y) (Math|Vector|BreakVector _returnvalue_2))
  ;[1 1 1] プレイヤーの移動に関する処理
  (bind _asthird_person_character (Utilities|Casting|CastToThirdPersonCharacter (Game|GetPlayerCharacter 0)))
  (if (Variables|/Game/BP/Player/ThirdPersonCharacter.ThirdPersonCharacter_C|Getpanelmove _asthird_person_character)
    (if (Variables|Default|Getmove)
      (Default|MakeTrail _asthird_person_character)
      (Variables|Default|Settime (+ (Variables|Default|Gettime) (Utilities|Time|GetWorldDeltaSeconds)))
      (bind _returnvalue_3 (Transformation|SetActorRotation _asthird_person_character (Math|Conversions|RotationFromXVector (Math|Vector|MakeVector _x _y 0.0))))
      (if _returnvalue_3
        (Transformation|SetActorLocation _asthird_person_character (Math|Vector|Lerp(Vector) _beginvec _returnvalue (/ (Variables|Default|Gettime) (/ (Variables|/Game/BP/Player/ThirdPersonCharacter.ThirdPersonCharacter_C|GetBeatDur _asthird_person_character) 2.0))) false false)
        (if (> (Variables|Default|Gettime) (/ (Variables|/Game/BP/Player/ThirdPersonCharacter.ThirdPersonCharacter_C|GetBeatDur _asthird_person_character) 2.0))
          (Pawn|Components|CharacterMovement|SetMovementMode (Variables|/Script/Engine.Character|GetCharacterMovement _asthird_person_character) "MOVE_Walking" 0)
          (Variables|/Game/BP/Player/ThirdPersonCharacter.ThirdPersonCharacter_C|SetIsDash _asthird_person_character false)
          (Variables|/Game/BP/Player/ThirdPersonCharacter.ThirdPersonCharacter_C|Setpanelmove _asthird_person_character false)
          (Variables|Default|Setmove false)
          (Variables|Default|Settime 0.0))))))

(event EventBeatFunction
  (bind _cylinder (Variables|Default|GetCylinder))
  ;[1 1 1] Beat Event
  (if (Utilities|IsValid (Variables|Default|GetNextPanel))
    (Variables|Default|Setchangemat (not (Variables|Default|Getchangemat)))
    (if (Variables|Default|Getchangemat)
      (Rendering|Material|SetMaterial _cylinder 0 "/Game/Resorce/Arrow/Material/arrow_Mat.arrow_Mat")
      (else
        (Rendering|Material|SetMaterial _cylinder 0 "/Game/Resorce/Arrow/Material/arrow2_Mat.arrow2_Mat")))
    (else
      (Rendering|Material|SetMaterial (Variables|Default|GetCylinder) 0 "/Engine/EngineDebugMaterials/BlackUnlitMaterial.BlackUnlitMaterial"))))

(event Collision|EventActorEndOverlap
  (params (OtherActor :type Actor%20Object%20Reference))
  (if (== OtherActor (Game|GetPlayerCharacter 0))
    (Variables|Default|SetRide false)))

(event EventBeginPlay
  (bind _returnvalue (Transformation|GetActorLocation))
  (bind _nextpanel (Variables|Default|GetNextPanel))
  (bind _returnvalue_2 (Transformation|GetActorLocation _nextpanel))
  (bind _returnvalue_3 (- _returnvalue _returnvalue_2))
  (bind (_x _y) (Math|Vector|BreakVector _returnvalue_3))
  (bind _returnvalue_4 (Math|Conversions|RotationFromXVector (Math|Vector|MakeVector _x _y 0.0)))
  (Transformation|SetWorldRotation (Variables|Default|GetCylinder) (Math|Rotator|MakeRotator (.roll _returnvalue_4) (.pitch _returnvalue_4) (+ (.yaw _returnvalue_4) -9e+01)) false false))

(event Input|ActionEvents|InputActionTeleport
  (params (Key :type Key%20Structure :default "None"))
  (bind _box (Variables|Default|GetBox))
  (:Pressed
    (if (and (Variables|Default|GetRide) (Utilities|IsValid (Variables|Default|GetNextPanel)))
      (bind _asthird_person_character (Utilities|Casting|CastToThirdPersonCharacter (Game|GetPlayerCharacter 0)))
      (bind _istiming (Default|TimingJudg _asthird_person_character))
      (if _istiming
        (Variables|Default|Setbeginvec (Transformation|GetActorLocation _asthird_person_character))
        (Pawn|Components|CharacterMovement|DisableMovement (Variables|/Script/Engine.Character|GetCharacterMovement _asthird_person_character))
        (Variables|/Game/BP/Player/ThirdPersonCharacter.ThirdPersonCharacter_C|SetIsDash _asthird_person_character true)
        (Variables|/Game/BP/Player/ThirdPersonCharacter.ThirdPersonCharacter_C|Setpanelmove _asthird_person_character true)
        (Variables|Default|Setmove true)
        (Variables|Default|Settime 0.0)
        (Default|AddCombo _asthird_person_character)
        (else
          ;[1 1 1] 当たり判定を一時的に消す
          (Collision|SetCollisionEnabled _box "NoCollision")
          (Utilities|FlowControl|Delay 1.0)
          (Collision|SetCollisionEnabled _box "QueryOnly"))))))

(event Input|ActionEvents|InputActionDash
  (params (Key :type Key%20Structure :default "None"))
  (bind _box (Variables|Default|GetBox))
  (:Pressed
    (if (and (Variables|Default|GetRide) (Utilities|IsValid (Variables|Default|GetNextPanel)))
      (bind _asthird_person_character (Utilities|Casting|CastToThirdPersonCharacter (Game|GetPlayerCharacter 0)))
      (bind _istiming (Default|TimingJudg _asthird_person_character))
      (if _istiming
        (Variables|Default|Setbeginvec (Transformation|GetActorLocation _asthird_person_character))
        (Pawn|Components|CharacterMovement|DisableMovement (Variables|/Script/Engine.Character|GetCharacterMovement _asthird_person_character))
        (Variables|/Game/BP/Player/ThirdPersonCharacter.ThirdPersonCharacter_C|SetIsDash _asthird_person_character true)
        (Variables|/Game/BP/Player/ThirdPersonCharacter.ThirdPersonCharacter_C|Setpanelmove _asthird_person_character true)
        (Variables|Default|Setmove true)
        (Variables|Default|Settime 0.0)
        (Default|AddCombo _asthird_person_character)
        (else
          ;[1 1 1] 当たり判定を一時的に消す
          (Collision|SetCollisionEnabled _box "NoCollision")
          (Utilities|FlowControl|Delay 1.0)
          (Collision|SetCollisionEnabled _box "QueryOnly"))))))

(fn ConstructionScript)