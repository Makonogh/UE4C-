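; BP_Rock is a destructible rock actor that spawns an enlarged explosion effect when its destructible mesh fractures.
; BeginPlay binds the mesh's fracture event, and a DoOnce limits the attached emitter to the first break.
; BeatFunction restarts a timeline whose track feeds the scale input of AddActorLocalTransform on each update.
; PlayerAttack and RockBeatEvent are empty stubs, and a steam emitter spawn is left unconnected.
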(event Custom|Custom
  (params (HitPoint :type Vector%20%28by%20ref%29) (HitDirection :type Vector%20%28by%20ref%29))
  (Utilities|FlowControl|DoOnce false
    (:Completed
      (Effects|SpawnEmitterAttached "/Game/StarterContent/Particles/P_Explosion.P_Explosion" (Variables|Default|GetSM_Rock_DM) "None" "0, 0, 0" "0, 0, 0" "5.000000,5.000000,5.000000"))))

(event Custom|RockBeatEvent)

(event EventBeginPlay
  (EventDispatchers|BindEventtoOnComponentFracture (Variables|Default|GetSM_Rock_DM) (delegate Custom|Custom)))

(event Collision|EventActorBeginOverlap
  (params (OtherActor :type Actor%20Object%20Reference)))

(event EventTick
  (params (DeltaSeconds :type Float%20%28single-precision%29)))

(event EventBeatFunction
  (bind _track_1 (Timeline|TimeLine PlayFromStart)
    (:Update
      (Class|Actor|AddActorLocalTransform (Math|Transform|MakeTransform "0, 0, 0" "0, 0, 0" _track_1) false false))))

(event EventPlayerAttack)

(fn ConstructionScript)