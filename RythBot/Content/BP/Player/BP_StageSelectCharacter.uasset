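; BP_StageSelectCharacter is the stage select character, which animates and flashes its lights in time with a musical beat.
; SetBPM stores the tempo, derives a beat duration from BPM and Divide, and sets the skeletal mesh's global animation rate to its inverse.
; Each BeatFunction call resets the beat timer value and toggles the eye and chest lights between yellow and red materials.
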(event EventSetBPM
  (params (BPM :type Float%20%28single-precision%29) (Divide :type Float%20%28single-precision%29))
  (Variables|Default|SetBPM BPM)
  (Variables|Default|SetDivide Divide)
  (bind _duration (CallFunction|GetBeatDuration BPM Divide))
  (bind _output_get (Variables|Default|SetBeatDur _duration))
  (Variables|Default|SetCurrent 0.0)
  (Variables|/Script/Engine.SkeletalMeshComponent|SetGlobalAnimRateScale (Variables|Default|GetSkeletalMesh) (/ 1.0 _output_get)))

(event EventBeatFunction
  (Variables|Default|SetCurrent 0.0)
  (if (Variables|Default|GetLight)
    (Rendering|Material|SetMaterial (Variables|Default|GetR_Eye_Light) 0 "/Game/Material/M_yello_Light.M_yello_Light")
    (Rendering|Material|SetMaterial (Variables|Default|GetL_Eye_Light) 0 "/Game/Material/M_yello_Light.M_yello_Light")
    (Rendering|Material|SetMaterial (Variables|Default|GetChest_Light) 0 "/Game/Material/M_yello_Light.M_yello_Light")
    (Variables|Default|SetLight false)
    (else
      (Rendering|Material|SetMaterial (Variables|Default|GetR_Eye_Light) 0 "/Game/Material/M_red_Light.M_red_Light")
      (Rendering|Material|SetMaterial (Variables|Default|GetL_Eye_Light) 0 "/Game/Material/M_red_Light.M_red_Light")
      (Rendering|Material|SetMaterial (Variables|Default|GetChest_Light) 0 "/Game/Material/M_red_Light.M_red_Light")
      (Variables|Default|SetLight true))))

(event EventTick
  (params (DeltaSeconds :type Float%20%28single-precision%29)))

(event EventBeginPlay)

(event Collision|EventActorBeginOverlap
  (params (OtherActor :type Actor%20Object%20Reference)))

(fn ConstructionScript)