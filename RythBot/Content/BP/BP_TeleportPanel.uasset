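; BP_TeleportPanel is a rhythm-timed panel that dashes the player to a linked NextPanel.
; Overlap sets a Ride flag; while it is set, a Dash or Teleport press that passes the character's timing judgment disables movement and adds a combo.
; Tick then turns the character toward NextPanel, makes a trail and lerps its location there over half a beat before restoring walking.
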(event EventBeginPlay)

(event Collision|EventActorBeginOverlap
  (params (OtherActor :type Actor%20Object%20Reference))
  (Variables|Default|Setride true))

(event EventTick
  (params (DeltaSeconds :type Float%20%28single-precision%29))
  (bind _beginvec (Variables|Default|Getbeginvec))
  (bind _nextpanel (Variables|Default|GetNextPanel))
  (bind _returnvalue (Transformation|GetActorLocation _nextpanel))
  (bind _returnvalue_2 (- _returnvalue _beginvec))
  (bind (_x _y) (Math|Vector|BreakVector _returnvalue_2))
  (bind _asthird_person_character (Utilities|Casting|CastToThirdPersonCharacter (Game|GetPlayerCharacter 0)))
  (if (Variables|/Game/BP/Player/ThirdPersonCharacter.ThirdPersonCharacter_C|Getpanelmove _asthird_person_character)
    (if (Variables|Default|Getmove)
      (Default|MakeTrail _asthird_person_character)
      (Variables|Default|Settime (+ (Variables|Default|Gettime) (Utilities|Time|GetWorldDeltaSeconds)))
      (bind _returnvalue_3 (Transformation|SetActorRotation _asthird_person_character (Math|Conversions|RotationFromXVector (Math|Vector|MakeVector _x _y 0.0))))
      (if _returnvalue_3
        (Transformation|SetActorLocation _asthird_person_character (Math|Vector|Lerp(Vector) _beginvec _returnvalue (/ (Variables|Default|Gettime) (/ (Variables|/Game/BP/Player/ThirdPersonCharacter.ThirdPersonCharacter_C|GetBeatDur _asthird_person_character) 2.0))) false false)
        (if (> (Variables|Default|Gettime) (/ (Variables|/Game/BP/Player/ThirdPersonCharacter.ThirdPersonCharacter_C|GetBeatDur _asthird_person_character) 2.0))
          (Pawn|Components|CharacterMovement|SetMovementMode (Variables|/Script/Engine.Character|GetCharacterMovement _asthird_person_character) "MOVE_Walking" 0)
          (Variables|/Game/BP/Player/ThirdPersonCharacter.ThirdPersonCharacter_C|SetIsDash _asthird_person_character false)
          (Variables|/Game/BP/Player/ThirdPersonCharacter.ThirdPersonCharacter_C|Setpanelmove _asthird_person_character false)
          (Variables|Default|Setmove false)
          (Variables|Default|Settime 0.0))))))

(event Collision|EventActorEndOverlap
  (params (OtherActor :type Actor%20Object%20Reference))
  (Variables|Default|Setride false))

(event Input|ActionEvents|InputActionTeleport
  (params (Key :type Key%20Structure :default "None"))
  (:Pressed
    (if (Variables|Default|Getride)
      (bind _asthird_person_character (Utilities|Casting|CastToThirdPersonCharacter (Game|GetPlayerCharacter 0)))
      (bind _istiming (Default|TimingJudg _asthird_person_character))
      (if _istiming
        (Variables|Default|Setbeginvec (Transformation|GetActorLocation _asthird_person_character))
        (Pawn|Components|CharacterMovement|DisableMovement (Variables|/Script/Engine.Character|GetCharacterMovement _asthird_person_character))
        (Variables|/Game/BP/Player/ThirdPersonCharacter.ThirdPersonCharacter_C|SetIsDash _asthird_person_character true)
        (Variables|/Game/BP/Player/ThirdPersonCharacter.ThirdPersonCharacter_C|Setpanelmove _asthird_person_character true)
        (Variables|Default|Setmove true)
        (Variables|Default|Settime 0.0)
        (Default|AddCombo _asthird_person_character)))))

(event Input|ActionEvents|InputActionDash
  (params (Key :type Key%20Structure :default "None"))
  (:Pressed
    (if (Variables|Default|Getride)
      (bind _asthird_person_character (Utilities|Casting|CastToThirdPersonCharacter (Game|GetPlayerCharacter 0)))
      (bind _istiming (Default|TimingJudg _asthird_person_character))
      (if _istiming
        (Variables|Default|Setbeginvec (Transformation|GetActorLocation _asthird_person_character))
        (Pawn|Components|CharacterMovement|DisableMovement (Variables|/Script/Engine.Character|GetCharacterMovement _asthird_person_character))
        (Variables|/Game/BP/Player/ThirdPersonCharacter.ThirdPersonCharacter_C|SetIsDash _asthird_person_character true)
        (Variables|/Game/BP/Player/ThirdPersonCharacter.ThirdPersonCharacter_C|Setpanelmove _asthird_person_character true)
        (Variables|Default|Setmove true)
        (Variables|Default|Settime 0.0)
        (Default|AddCombo _asthird_person_character)))))

(fn ConstructionScript)