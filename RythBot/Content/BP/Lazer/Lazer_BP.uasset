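; Rhythm-synced laser turret enemy that aims at the player and fires a damaging beam until the player's attack destroys it.
; Each BeatFunction call advances a four-stage cycle: two tracking the player, one blinking on the locked direction, one firing; SetBPM supplies the blink timing.
; Tick line traces set beam endpoints, and firing sends EnemyAttack_BPI damage through a DoOnce.
; PlayerAttack triggers an explosion, drops the blackened core with physics and stops Tick.
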(event EventBeginPlay
  (bind _returnvalue (Rendering|Material|CreateDynamicMaterialInstance (Variables|Default|GetLazer_PT) 0 "/Game/Material/Lazer_mat_Inst.Lazer_mat_Inst" "None" :!class /Script/Engine.PrimitiveComponent))
  (Variables|Default|SetLazerMaterialInst _returnvalue)
  (bind _returnvalue_2 (Rendering|Material|CreateDynamicMaterialInstance (Variables|Default|GetLazerCore_SM) 0 "/Game/Resorce/Enemy/Lazer/Texture/LazerCore_mat_Inst.LazerCore_mat_Inst" "None" :!class /Script/Engine.PrimitiveComponent))
  (Variables|Default|SetCoreMaterialInst _returnvalue_2))

(event Collision|EventActorBeginOverlap
  (params (OtherActor :type Actor%20Object%20Reference)))

(event EventTick
  (params (DeltaSeconds :type Float%20%28single-precision%29))
  (bind _lazercore_sm (Variables|Default|GetLazerCore_SM))
  (bind _lazercore_sm_2 (Variables|Default|GetLazerCore_SM))
  (bind _returnvalue (Transformation|GetWorldLocation _lazercore_sm_2))
  (bind _returnvalue_2 (Transformation|GetWorldLocation _lazercore_sm))
  (if (not (Variables|Default|GetIsDead))
    (Variables|Default|SetTime (+ DeltaSeconds (Variables|Default|GetTime)))
    (Transformation|AddLocalRotation (Variables|Default|GetLazerCore_SM) (Math|Rotator|MakeRotator 0.0 0.0 (* DeltaSeconds 4e+01)) false true)
    (switch int (Variables|Default|GetAttackStage)
      (:0
        (bind _outhit (Collision|LineTraceForObjects (Transformation|GetWorldLocation (Variables|Default|GetLazerCore_SM)) (Transformation|GetActorLocation (Game|GetPlayerCharacter 0)) (Utilities|Array|MakeArray "ObjectTypeQuery1" "ObjectTypeQuery2" "ObjectTypeQuery4" "ObjectTypeQuery6" "ObjectTypeQuery3") false 0 "None" :!label _label))
        (if (.bBlockingHit (Collision|BreakHitResult _outhit))
          (Class|ParticleSystemComponent|SetBeamTargetPoint (Variables|Default|GetLazer_PT) 0 (.Location (Collision|BreakHitResult _outhit)))
          (Variables|Default|SetCurrentLazerVector (.Location (Collision|BreakHitResult _outhit)))
          (else
            (Class|ParticleSystemComponent|SetBeamTargetPoint (Variables|Default|GetLazer_PT) 0 (.TraceEnd (Collision|BreakHitResult _outhit)))
            (Variables|Default|SetCurrentLazerVector (.TraceEnd (Collision|BreakHitResult _outhit))))))
      (:1
        (goto _label))
      (:2
        (Rendering|Material|SetScalarParameterValue (Variables|Default|GetLazerMaterialInst) "Alpha" (Math|Float|Fraction (/ (Variables|Default|GetTime) (* (Variables|Default|GetDuration) 0.1))) :!class /Script/Engine.MaterialInstanceDynamic)
        (bind _outhit_2 (Collision|LineTraceForObjects (Transformation|GetWorldLocation (Variables|Default|GetLazerCore_SM)) (+ _returnvalue (* (Math|Vector|Normalize (- (Variables|Default|GetCurrentLazerVector) _returnvalue)) 5e+03)) (Utilities|Array|MakeArray "ObjectTypeQuery1" "ObjectTypeQuery2" "ObjectTypeQuery4" "ObjectTypeQuery6" "ObjectTypeQuery3") false 0 "None"))
        (if (.bBlockingHit (Collision|BreakHitResult _outhit_2))
          (Class|ParticleSystemComponent|SetBeamTargetPoint (Variables|Default|GetLazer_PT) 0 (.Location (Collision|BreakHitResult _outhit_2)))
          (goto _label_2 Reset)
          (else
            (Class|ParticleSystemComponent|SetBeamTargetPoint (Variables|Default|GetLazer_PT) 0 (.TraceEnd (Collision|BreakHitResult _outhit_2)))
            (goto _label_2 Reset))))
      (:3
        (Utilities|FlowControl|Sequence
          (:then_0
            (Utilities|FlowControl|DoOnce false
              (:Completed
                (Components|Activation|Activate (Variables|Default|GetLazerAttack_PT) true))))
          (:then_1
            (bind _outhit_3 (Collision|LineTraceForObjects (Transformation|GetWorldLocation (Variables|Default|GetLazerCore_SM)) (+ _returnvalue_2 (* (Math|Vector|Normalize (- (Variables|Default|GetCurrentLazerVector) _returnvalue_2)) 5e+03)) (Utilities|Array|MakeArray "ObjectTypeQuery1" "ObjectTypeQuery2" "ObjectTypeQuery4" "ObjectTypeQuery6" "ObjectTypeQuery3") false 0 "None"))
            (if (.bBlockingHit (Collision|BreakHitResult _outhit_3))
              (Class|ParticleSystemComponent|SetBeamTargetPoint (Variables|Default|GetLazerAttack_PT) 0 (.Location (Collision|BreakHitResult _outhit_3)))
              (Class|ParticleSystemComponent|SetBeamTargetPoint (Variables|Default|GetLazer_PT) 0 (.Location (Collision|BreakHitResult _outhit_3)))
              ;[1 1 1] 攻撃
              (if (Utilities|DoesObjectImplementInterface (.HitActor (Collision|BreakHitResult _outhit_3)) "/Game/BP/Interface/EnemyAttack_BPI.EnemyAttack_BPI_C")
                (Utilities|FlowControl|DoOnce false :!label _label_2
                  (:Completed
                    (Class|EnemyAttackBPI|EnemyAttack(Message) (.HitActor (Collision|BreakHitResult _outhit_3)) 2 (.Location (Collision|BreakHitResult _outhit_3))))))
              (else
                (Class|ParticleSystemComponent|SetBeamTargetPoint (Variables|Default|GetLazerAttack_PT) 0 (.TraceEnd (Collision|BreakHitResult _outhit_3)))
                (Class|ParticleSystemComponent|SetBeamTargetPoint (Variables|Default|GetLazer_PT) 0 (.TraceEnd (Collision|BreakHitResult _outhit_3)))))))))))

(event EventBeatFunction
  (if (not (Variables|Default|GetIsDead))
    (if (Variables|Default|GetActive)
      (Variables|Default|SetAttackStage (Math|Integer|%(Integer) (+ (Variables|Default|GetAttackStage) 1) 4))
      (Variables|Default|SetTime 0.0)
      (Rendering|SetVisibility (Variables|Default|GetLazer_PT) true false)
      (Rendering|Material|SetScalarParameterValue (Variables|Default|GetLazerMaterialInst) "Alpha" 1.0 :!class /Script/Engine.MaterialInstanceDynamic)
      (Components|Activation|Deactivate (Variables|Default|GetLazerAttack_PT))
      (Utilities|FlowControl|DoOnce false) ; enters at Reset
      (else
        (Variables|Default|SetActive true)
        (Variables|Default|SetAttackStage 0)))))

(event EventSetBPM
  (params (BPM :type Float%20%28single-precision%29) (Divide :type Float%20%28single-precision%29))
  (Variables|Default|SetDuration Divide))

(event EventPlayerAttack
  ;[1 1 1] 攻撃された
  (Utilities|FlowControl|DoOnce false
    (:Completed
      (Effects|SpawnEmitteratLocation "/Game/Resorce/StarterContent/Particles/P_Explosion.P_Explosion" (Transformation|GetWorldLocation (Variables|Default|GetLazerCore_SM)) "0, 0, 0" "2.000000,2.000000,2.000000")
      (Physics|SetSimulatePhysics (Variables|Default|GetLazerCore_SM) true)
      (Variables|Default|SetIsDead true)
      (Components|DestroyComponent (Variables|Default|GetLazer_PT))
      (Components|DestroyComponent (Variables|Default|GetLazerAttack_PT))
      (Rendering|Material|SetVectorParameterValue (Variables|Default|GetCoreMaterialInst) "Color" (Utilities|Struct|MakeLinearColor 0.0 0.0 0.0 1.0) :!class /Script/Engine.MaterialInstanceDynamic)
      (Actor|Tick|SetActorTickEnabled false))))

(fn ConstructionScript)