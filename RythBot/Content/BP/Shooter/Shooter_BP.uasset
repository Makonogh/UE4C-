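; Shooter enemy that wanders until it sees the player, then faces them and fires on the beat.
; Each tick a line trace sets sight and target rotation, steering movement toward a point 600 units horizontally from the player or along a random heading.
; BeatFunction alternates between readying and spending a shot, spawning a bullet and particles when the player is visible.
; PlayerAttack turns on physics, fractures the destructible mesh once and destroys the actor seven seconds later.
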(event EventBeginPlay
  (Variables|Default|SetMoveVector (* (Class|KismetMathLibrary|VectorForward) 1e+02))
  (Variables|Default|SetRotateSpeed 5.0))

(event Collision|EventActorBeginOverlap
  (params (OtherActor :type Actor%20Object%20Reference)))

(event EventTick
  (params (DeltaSeconds :type Float%20%28single-precision%29))
  (if (Variables|Default|GetIsDead)
    (bind _output_get (Variables|Default|SetDeadTime (+ (Variables|Default|GetDeadTime) DeltaSeconds)))
    (if (>= _output_get 7.0)
      (Actor|DestroyActor))
    (else
      (CallFunction|RotateUpdate)
      (CallFunction|MoveUpdate DeltaSeconds)
      (Transformation|SetWorldRotation (Variables|Default|GetShooter_DM) (Math|Interpolation|RInterpTo (Transformation|GetWorldRotation (Variables|Default|GetShooter_DM)) (Variables|Default|GetTargetRot) DeltaSeconds (Variables|Default|GetRotateSpeed)) false false))))

(event EventBeatFunction
  (bind _scene (Variables|Default|GetScene))
  (bind _returnvalue (Transformation|GetWorldTransform _scene))
  (bind (_location _rotation _scale) (Math|Transform|BreakTransform _returnvalue))
  ;[1 1 1] 攻撃
  (if (not (Variables|Default|GetIsDead))
    (if (Variables|Default|GetCanShoot)
      (Variables|Default|SetCanShoot false)
      (if (Variables|Default|GetIsPlayerInSight)
        (Game|SpawnActorfromClass "/Game/BP/Shooter/ShooterBullet.ShooterBullet_C" _returnvalue "AdjustIfPossibleButDontSpawnIfColliding" 0 0)
        (Effects|SpawnEmitteratLocation "/Game/Particle/ShootWave_PT.ShootWave_PT" _location _rotation _scale))
      (else
        (Variables|Default|SetCanShoot true)))))

(event EventPlayerAttack
  ;[1 1 1] 攻撃された
  (Utilities|FlowControl|DoOnce false
    (:Completed
      (Physics|SetSimulatePhysics (Variables|Default|GetShooter_DM) true)
      (Physics|SetEnableGravity (Variables|Default|GetShooter_DM) true)
      (Class|DestructibleComponent|ApplyRadiusDamage (Variables|Default|GetShooter_DM) 1.0 (Transformation|GetWorldLocation (Variables|Default|GetShooter_DM)) 0.0 0.0 true)
      (Variables|Default|SetIsDead true))))

(fn ConstructionScript)

(fn MoveUpdate
  (params (DeltaTime :type Float%20%28single-precision%29))
  (bind _returnvalue (Game|GetPlayerCharacter 0))
  (bind _shooter_dm (Variables|Default|GetShooter_DM))
  (bind _returnvalue_2 (Transformation|GetWorldLocation _shooter_dm))
  (bind _capsulecomponent (Variables|/Script/Engine.Character|GetCapsuleComponent _returnvalue))
  (bind (_x _y) (Math|Vector|BreakVector _returnvalue_2))
  (bind _returnvalue_3 (Transformation|GetWorldLocation _capsulecomponent))
  (bind (_x_2 _y_2) (Math|Vector|BreakVector _returnvalue_3))
  (if (Variables|Default|GetIsPlayerInSight)
    (bind _output_get (LocalVariables|SetPlayerVec (- (Math|Vector|MakeVector _x _y 0.0) (Math|Vector|MakeVector _x_2 _y_2 0.0))))
    (bind _output_get_2 (Variables|Default|SetMoveVector (* (Math|Vector|GetForwardVector (Class|KismetMathLibrary|RInterptoConstant (Math|Conversions|RotationFromXVector (Variables|Default|GetMoveVector)) (Math|Conversions|RotationFromXVector (- (+ (* (Math|Vector|Normalize _output_get) 6e+02) _returnvalue_3) _returnvalue_2)) DeltaTime 5e+01)) 1e+02)))
    (Transformation|AddWorldOffset (Variables|Default|GetShooter_DM) (* _output_get_2 DeltaTime) true false)
    (else
      (bind _output_get_3 (Variables|Default|SetMoveVector (Math|Vector|RotateVector (Variables|Default|GetMoveVector) (Math|Rotator|MakeRotator 0.0 0.0 (Math|Random|RandomFloatinRange (* DeltaTime -3e+02) (* DeltaTime 3e+02))))))
      (Transformation|AddWorldOffset (Variables|Default|GetShooter_DM) (* _output_get_3 DeltaTime) true false))))

(fn RotateUpdate
  (bind _returnvalue (Game|GetPlayerCharacter 0))
  (bind _shooter_dm (Variables|Default|GetShooter_DM))
  (bind _returnvalue_2 (Transformation|GetWorldLocation _shooter_dm))
  (bind _capsulecomponent (Variables|/Script/Engine.Character|GetCapsuleComponent _returnvalue))
  (bind _returnvalue_3 (Transformation|GetWorldLocation _capsulecomponent))
  (bind _outhit (Collision|LineTraceForObjects _returnvalue_2 (+ _returnvalue_2 (* (- _returnvalue_3 _returnvalue_2) 1e+03)) (Utilities|Array|MakeArray "ObjectTypeQuery1" "ObjectTypeQuery2" "ObjectTypeQuery3" "ObjectTypeQuery4" "ObjectTypeQuery6") false 0 "None"))
  (if (== (.HitActor (Collision|BreakHitResult _outhit)) _returnvalue)
    (Variables|Default|SetTargetRot (Math|Conversions|RotationFromXVector (- _returnvalue_3 _returnvalue_2)))
    (Variables|Default|SetIsPlayerInSight true)
    (Variables|Default|SetRotateSpeed 5e+01)
    (else
      (Variables|Default|SetTargetRot (Math|Conversions|RotationFromXVector (Variables|Default|GetMoveVector)))
      (Variables|Default|SetRotateSpeed 5.0)
      (if (Variables|Default|GetIsPlayerInSight)
        (Variables|Default|SetMoveVector (* (Class|KismetMathLibrary|VectorNormal2D (Variables|Default|GetMoveVector) 0.0001) 1e+02))
        (Variables|Default|SetIsPlayerInSight false)))))