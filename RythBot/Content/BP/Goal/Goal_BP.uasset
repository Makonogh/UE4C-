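; Level goal actor that pulses to the music and ends the stage when the player enters its capsule.
; Dynamic material instances on wave and pillar meshes animate a panning position over two beats, restarting on every second beat call.
; Player overlap disables input, sends PlayerAttackMessage to all interface implementers and plays a level sequence.
; CallResultUI re-enables character input, switches to UI-only mode and shows the result widget carrying the next level name.
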(event OnComponentBeginOverlap(Capsule)
  (params (OverlappedComponent :type Primitive%20Component%20Object%20Reference) (OtherActor :type Actor%20Object%20Reference) (OtherComp :type Primitive%20Component%20Object%20Reference) (OtherBodyIndex :type Integer) (bFromSweep :type Boolean) (SweepResult :type Hit%20Result%20Structure%20%28by%20ref%29))
  (bind _returnvalue (Game|GetPlayerCharacter 0))
  (if (== OtherActor _returnvalue)
    (Input|DisableInput _returnvalue (Game|GetPlayerController 0))
    (bind _outactors (Actor|GetAllActorswithInterface "/Game/BP/Interface/PlayerAttack_BPI.PlayerAttack_BPI_C"))
    (for _array_element _outactors
      (Class|PlayerAttackBPI|PlayerAttack(Message) _array_element))
    (Sequencer|Player|Play (Variables|/Script/LevelSequence.LevelSequenceActor|GetSequencePlayer (Variables|Default|GetSequence)) :!class /Script/MovieScene.MovieSceneSequencePlayer)))

(event Custom|CallResultUI
  (bind _returnvalue (Game|GetPlayerController 0))
  (Variables|/Script/Engine.PlayerController|SetbShowMouseCursor _returnvalue true)
  (Input|SetInputModeUIOnly _returnvalue 0 "DoNotLock")
  (Input|EnableInput (Game|GetPlayerCharacter 0) _returnvalue)
  (UserInterface|Viewport|AddtoViewport (Variables|Default|GetResultUI) 10000))

(event EventBeginPlay
  (bind _returnvalue (Rendering|Material|CreateDynamicMaterialInstance (Variables|Default|GetStaticMesh) 0 "/Game/Material/SimplePanMaterial.SimplePanMaterial" "None" :!class /Script/Engine.PrimitiveComponent))
  (Variables|Default|SetWaveMaterialInstance _returnvalue)
  (bind _returnvalue_2 (Rendering|Material|CreateDynamicMaterialInstance (Variables|Default|GetStaticMesh1) 0 "/Game/Material/SimplePanMaterial.SimplePanMaterial" "None" :!class /Script/Engine.PrimitiveComponent))
  (Variables|Default|SetPillarMaterialInstance _returnvalue_2)
  (Variables|Default|SetTime 0.0)
  (Rendering|Material|SetScalarParameterValue (Variables|Default|GetWaveMaterialInstance) "Position" 0.0 :!class /Script/Engine.MaterialInstanceDynamic)
  (Rendering|Material|SetVectorParameterValue (Variables|Default|GetWaveMaterialInstance) "Color" (Utilities|Struct|MakeLinearColor 0.0 1.0 5.0 1.0) :!class /Script/Engine.MaterialInstanceDynamic)
  (Rendering|Material|SetScalarParameterValue (Variables|Default|GetPillarMaterialInstance) "Position" 0.0 :!class /Script/Engine.MaterialInstanceDynamic)
  (Rendering|Material|SetScalarParameterValue (Variables|Default|GetPillarMaterialInstance) "LineCount" 2e+01 :!class /Script/Engine.MaterialInstanceDynamic)
  (Rendering|Material|SetVectorParameterValue (Variables|Default|GetPillarMaterialInstance) "Color" (Utilities|Struct|MakeLinearColor 0.0 1.0 5.0 1.0) :!class /Script/Engine.MaterialInstanceDynamic)
  (bind _returnvalue_3 (UserInterface|CreateWidget "/Game/BP/UI/ResultUI.ResultUI_C"))
  (Variables|Default|SetResultUI _returnvalue_3)
  (Default|SetNextLevel (Variables|Default|GetResultUI) (Variables|Default|GetNextLevelName)))

(event EventTick
  (params (DeltaSeconds :type Float%20%28single-precision%29))
  (bind _output_get (Variables|Default|SetTime (Math|Float|Min(Float) (+ DeltaSeconds (Variables|Default|GetTime)) (Variables|Default|GetDuration))))
  (Rendering|Material|SetScalarParameterValue (Variables|Default|GetWaveMaterialInstance) "Position" (/ _output_get (Variables|Default|GetDuration)) :!class /Script/Engine.MaterialInstanceDynamic)
  (Rendering|Material|SetScalarParameterValue (Variables|Default|GetPillarMaterialInstance) "Position" (/ (/ _output_get (Variables|Default|GetDuration)) 1e+01) :!class /Script/Engine.MaterialInstanceDynamic))

(event EventSetBPM
  (params (BPM :type Float%20%28single-precision%29) (Divide :type Float%20%28single-precision%29))
  (bind _duration (CallFunction|GetBeatDuration BPM Divide))
  (Variables|Default|SetDuration (* _duration 2.0)))

(event EventBeatFunction
  (if (Variables|Default|GetWait)
    (Variables|Default|SetTime 0.0)
    (Variables|Default|SetWait false)
    (else
      (Variables|Default|SetWait true))))

(fn ConstructionScript)