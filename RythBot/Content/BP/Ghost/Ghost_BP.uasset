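; Ghost enemy that attacks in time with the music while it has line of sight to the player.
; Every other beat advances a cycle: vanish, reappear near the player, curve-driven homing body blow, random drift.
; Contact during the blow damages the player; a player attack destroys the ghost and sends a death message to its Door.
; Per-frame movement feeds leg material offsets so the legs react to motion.
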(event OnComponentHit(Capsule)
  (params (HitComponent :type Primitive%20Component%20Object%20Reference) (OtherActor :type Actor%20Object%20Reference) (OtherComp :type Primitive%20Component%20Object%20Reference) (NormalImpulse :type Vector :default "0, 0, 0") (Hit :type Hit%20Result%20Structure%20%28by%20ref%29))
  ;[1 1 1] 攻撃
  (if (and (== OtherComp (Variables|/Script/Engine.Character|GetCapsuleComponent (Game|GetPlayerCharacter 0))) (== (Variables|Default|GetState) 2))
    (Class|EnemyAttackBPI|EnemyAttack(Message) OtherActor 1 (Transformation|GetWorldLocation (Variables|Default|GetGhost)))))

(event EventBeginPlay
  ;[1 1 1] 初期化
  (bind _returnvalue (Rendering|Material|CreateDynamicMaterialInstance (Variables|Default|GetGhost) 1 "/Game/Resorce/Enemy/Ghost/Texture/Leg.Leg" "None" :!class /Script/Engine.PrimitiveComponent))
  (Variables|Default|SetLegMaterialInstance _returnvalue)
  (Variables|Default|SetPrevLocation (Transformation|GetActorLocation)))

(event EventBeatFunction
  (bind _output_get (Variables|Default|SetWaitBeat (not (Variables|Default|GetWaitBeat))))
  (if _output_get
    (if (Variables|Default|GetIsActive)
      (bind _result (Math|Integer|IncrementInt (Variables|Default|GetState))
        (:%20%20
          (Variables|Default|SetState (Math|Integer|%(Integer) _result 4))
          (Variables|Default|SetIsExecuted false)
          (Variables|Default|SetTime 0.0)
          (if (== (Variables|Default|GetState) 0)
            (CallFunction|CheckPlayeronSight)))))))

(event EventTick
  (params (DeltaSeconds :type Float%20%28single-precision%29))
  (CallFunction|LegUpdate DeltaSeconds)
  (Variables|Default|SetPrevLocation (Transformation|GetWorldLocation (Variables|Default|GetGhost)))
  (Variables|Default|SetTime (Math|Float|Min(Float) (+ (Variables|Default|GetTime) DeltaSeconds) (Variables|Default|GetBeatDuration)))
  (if (Variables|Default|GetIsActive)
    (switch int (Variables|Default|GetState)
      (:0
        (CallFunction|Disappear))
      (:1
        (CallFunction|Appear))
      (:2
        (CallFunction|BodyBlow))
      (:3
        (CallFunction|Wait)))
    (else
      (CallFunction|CheckPlayeronSight))))

(event EventSetBPM
  (params (BPM :type Float%20%28single-precision%29) (Divide :type Float%20%28single-precision%29))
  (bind _duration (CallFunction|GetBeatDuration BPM Divide))
  (Variables|Default|SetBeatDuration (* _duration 2.0))
  (Variables|Default|SetTime 0.0))

(event EventPlayerAttack
  (bind _ghost (Variables|Default|GetGhost))
  (bind _returnvalue (Transformation|GetWorldTransform _ghost))
  ;[1 1 1] 攻撃を受けた
  (Utilities|FlowControl|DoOnce false
    (:Completed
      (Niagara|SpawnSystematLocation "/Game/Particle/GhostDead/GhostDead_NS.GhostDead_NS" (.location _returnvalue) (.rotation _returnvalue) (.scale _returnvalue))
      (Class|DeathFlag|Death(Message) (Variables|Default|GetDoor))
      (Actor|DestroyActor))))

(fn ConstructionScript)

(fn LegUpdate
  (params (DeltaTime :type Float%20%28single-precision%29))
  (bind _returnvalue (* DeltaTime 2e+01))
  (bind _prevlocation (Variables|Default|GetPrevLocation))
  (bind _ghost (Variables|Default|GetGhost))
  (bind _returnvalue_2 (Transformation|GetWorldLocation _ghost))
  (bind _returnvalue_3 (- _prevlocation _returnvalue_2))
  (bind _returnvalue_4 (/ _returnvalue_3 _returnvalue))
  (Rendering|Material|SetScalarParameterValue (Variables|Default|GetLegMaterialInstance) "OffsetX" (.x _returnvalue_4) :!class /Script/Engine.MaterialInstanceDynamic)
  (Rendering|Material|SetScalarParameterValue (Variables|Default|GetLegMaterialInstance) "OffsetY" (.y _returnvalue_4) :!class /Script/Engine.MaterialInstanceDynamic))

(fn CheckPlayeronSight
  (bind _returnvalue (Game|GetPlayerCharacter 0))
  (bind _outhit (Collision|LineTraceForObjects (Transformation|GetWorldLocation (Variables|Default|GetGhost)) (Transformation|GetWorldLocation (Variables|/Script/Engine.Character|GetCapsuleComponent _returnvalue)) (Utilities|Array|MakeArray "ObjectTypeQuery1" "ObjectTypeQuery2" "ObjectTypeQuery3" "ObjectTypeQuery4" "ObjectTypeQuery6") true 0 "None"))
  (bind _output_get (Variables|Default|SetIsActive (== _returnvalue (.HitActor (Collision|BreakHitResult _outhit)))))
  (if (not _output_get)
    (Variables|Default|SetState 0)))

(fn Disappear
  (bind _ghost (Variables|Default|GetGhost))
  (bind _returnvalue (Transformation|GetWorldTransform _ghost))
  (bind (_location _rotation _scale) (Math|Transform|BreakTransform _returnvalue))
  (if (not (Variables|Default|GetIsExecuted))
    (Rendering|SetVisibility (Variables|Default|GetGhost) false false)
    (Niagara|SpawnSystematLocation "/Game/Particle/GhostDisAppear/Ghost_NS.Ghost_NS" _location _rotation _scale)
    (Variables|Default|SetIsExecuted true)))

(fn Appear
  (bind _ghost (Variables|Default|GetGhost))
  (bind _returnvalue (Transformation|GetWorldTransform _ghost))
  (bind (_location _rotation _scale) (Math|Transform|BreakTransform _returnvalue))
  (if (Variables|Default|GetIsExecuted)
    (Utilities|IsValid (Variables|Default|GetParticle)
      (:Is%20Not%20Valid
        (Rendering|SetVisibility (Variables|Default|GetGhost) true false)))
    (else
      (Variables|Default|SetMoveVector (Math|Vector|RotateVector (Class|KismetMathLibrary|VectorForward) (Math|Rotator|MakeRotator 0.0 0.0 (Math|Random|RandomFloatinRange 0.0 3.6e+02))))
      (Transformation|SetWorldLocation (Variables|Default|GetGhost) (+ (Transformation|GetWorldLocation (Variables|/Script/Engine.Character|GetCapsuleComponent (Game|GetPlayerCharacter 0))) (* (Variables|Default|GetMoveVector) (Math|Random|RandomFloatinRange -3e+02 -7e+02)) (Math|Vector|MakeVector 0.0 0.0 8e+01)) false true)
      (Transformation|SetWorldRotation (Variables|Default|GetGhost) (Math|Conversions|RotationFromXVector (Variables|Default|GetMoveVector)) false false)
      (bind _returnvalue_2 (Niagara|SpawnSystematLocation "/Game/Particle/GhostAppear/GhostAppear_NS.GhostAppear_NS" _location _rotation _scale))
      (Variables|Default|SetParticle _returnvalue_2)
      (Variables|Default|SetIsExecuted true)
      (Variables|Default|SetPrevLocation (Transformation|GetWorldLocation (Variables|Default|GetGhost))))))

(fn BodyBlow
  (bind _beatduration (Variables|Default|GetBeatDuration))
  (bind _time (Variables|Default|GetTime))
  (bind _movecurve (Variables|Default|GetMoveCurve))
  (bind _returnvalue (/ _time _beatduration))
  (bind _returnvalue_2 (Math|Curves|GetFloatValue _movecurve _returnvalue))
  (if (Variables|Default|GetIsExecuted)
    (CallFunction|HomingtoPlayer)
    (Transformation|AddWorldOffset (Variables|Default|GetGhost) (* (Variables|Default|GetMoveVector) (- _returnvalue_2 (Variables|Default|GetPrevDelta))) false true)
    (Variables|Default|SetPrevDelta _returnvalue_2)
    (else
      (Variables|Default|SetMoveVector (* (Variables|Default|GetMoveVector) 1.2e+03))
      (Variables|Default|SetPrevDelta 0.0)
      (Variables|Default|SetIsExecuted true))))

(fn Wait
  (if (Variables|Default|GetIsExecuted)
    (Transformation|AddWorldOffset (Variables|Default|GetGhost) (* (Variables|Default|GetMoveVector) (Utilities|Time|GetWorldDeltaSeconds)) false true)
    (else
      (bind _output_get (Variables|Default|SetMoveVector (* (Math|Vector|RotateVector (Class|KismetMathLibrary|VectorForward) (Math|Rotator|MakeRotator 0.0 0.0 (Math|Random|RandomFloatinRange 0.0 3.6e+02))) (Math|Random|RandomFloatinRange 2e+02 3e+02))))
      (Transformation|SetWorldRotation (Variables|Default|GetGhost) (Math|Conversions|RotationFromXVector _output_get) false true)
      (Variables|Default|SetIsExecuted true))))

(fn HomingtoPlayer
  (Variables|Default|SetMoveVector (* (Math|Rotator|GetRotationXVector (Class|KismetMathLibrary|RInterptoConstant (Math|Conversions|RotationFromXVector (Variables|Default|GetMoveVector)) (Math|Conversions|RotationFromXVector (Math|Vector|Normalize (- (+ (Transformation|GetWorldLocation (Variables|/Script/Engine.Character|GetCapsuleComponent (Game|GetPlayerCharacter 0))) "0, 0,80.000000") (Transformation|GetWorldLocation (Variables|Default|GetGhost))))) (Utilities|Time|GetWorldDeltaSeconds) 1.5e+02)) 1.2e+03))
  (Transformation|SetWorldRotation (Variables|Default|GetGhost) (Class|KismetMathLibrary|RInterptoConstant (Math|Conversions|RotationFromXVector (Variables|Default|GetMoveVector)) (Math|Conversions|RotationFromXVector (Math|Vector|Normalize (- (+ (Transformation|GetWorldLocation (Variables|/Script/Engine.Character|GetCapsuleComponent (Game|GetPlayerCharacter 0))) "0, 0,80.000000") (Transformation|GetWorldLocation (Variables|Default|GetGhost))))) (Utilities|Time|GetWorldDeltaSeconds) 1.5e+02) false false))