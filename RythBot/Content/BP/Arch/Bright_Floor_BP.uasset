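; Bright floor Blueprint whose plane surface changes brightness in response to a beat event.
; On BeginPlay it creates a dynamic material instance on the plane and applies its two color variables and tile size.
; Each BeatFunction call restarts the BeatLine timeline, which feeds the material's Bright parameter to animate the pulse.
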(event EventBeginPlay
  ;[1 1 1] 初期化
  (bind _returnvalue (Rendering|Material|CreateDynamicMaterialInstance (Variables|Default|GetPlane) 0 "/Game/Material/BrightFloor_mat_Inst.BrightFloor_mat_Inst" "None" :!class /Script/Engine.PrimitiveComponent))
  (Variables|Default|SetMatInstance _returnvalue)
  (Rendering|Material|SetVectorParameterValue (Variables|Default|GetMatInstance) "Color1" (Variables|Default|GetColor1) :!class /Script/Engine.MaterialInstanceDynamic)
  (Rendering|Material|SetVectorParameterValue (Variables|Default|GetMatInstance) "Color2" (Variables|Default|GetColor2) :!class /Script/Engine.MaterialInstanceDynamic)
  (Rendering|Material|SetScalarParameterValue (Variables|Default|GetMatInstance) "TileSize" (Variables|Default|GetTileSize) :!class /Script/Engine.MaterialInstanceDynamic))

(event EventBeatFunction
  ;[1 1 1] Beat Event
  (bind _bright (Timeline|BeatLine PlayFromStart)
    (:Update
      (Rendering|Material|SetScalarParameterValue (Variables|Default|GetMatInstance) "Bright" _bright :!class /Script/Engine.MaterialInstanceDynamic))))

(fn ConstructionScript)