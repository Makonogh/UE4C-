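; BP_EnemyCheck is an actor that removes itself once every Lazer_BP enemy in the level is dead.
; Each Tick, while the player ThirdPersonCharacter's IsGoodTiming flag is set, it gathers all Lazer_BP actors and checks their IsDead flags.
; If none are alive, including when none exist, it sets a Once guard and destroys itself.
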(event EventBeginPlay
  (Variables|Default|Setonce false))

(event Collision|EventActorBeginOverlap
  (params (OtherActor :type Actor%20Object%20Reference)))

(event EventTick
  (params (DeltaSeconds :type Float%20%28single-precision%29))
  (if (not (Variables|Default|Getonce))
    (bind _asthird_person_character (Utilities|Casting|CastToThirdPersonCharacter (Game|GetPlayerCharacter 0)))
    (if (Variables|/Game/BP/ThirdPersonCharacter.ThirdPersonCharacter_C|GetIsGoodTiming _asthird_person_character)
      (bind _outactors (Actor|GetAllActorsOfClass "/Game/BP/Lazer/Lazer_BP.Lazer_BP_C"))
      (Variables|Default|SetAlldead true)
      (for _array_element _outactors
        (if (not (Variables|/Game/BP/Lazer/Lazer_BP.Lazer_BP_C|GetIsDead _array_element))
          (Variables|Default|SetAlldead false)))
      (if (Variables|Default|GetAlldead)
        (Variables|Default|Setonce true)
        (Actor|DestroyActor)))))

(fn ConstructionScript)