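; Beat-synced spring enemy that hops between targets and damages the player.
; Each beat restarts the timer and notifies its AI controller; ExecuteJump and SetIdle switch movement state.
; Tick lerps jumps over one beat with a sine arc and curve-driven spring offset, while capsule overlap deals damage once per beat.
; A player attack shatters both destructible meshes with radial damage, unpossesses it and disables collision before delayed destruction.
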(event OnComponentBeginOverlap(CapsuleComponent)
  (params (OverlappedComponent :type Primitive%20Component%20Object%20Reference) (OtherActor :type Actor%20Object%20Reference) (OtherComp :type Primitive%20Component%20Object%20Reference) (OtherBodyIndex :type Integer) (bFromSweep :type Boolean) (SweepResult :type Hit%20Result%20Structure%20%28by%20ref%29))
  ;[1 1 1] 攻撃する
  (Utilities|FlowControl|DoOnce false
    (:Completed
      (if (and (== OtherComp (Variables|/Script/Engine.Character|GetCapsuleComponent (Game|GetPlayerCharacter 0))) (Variables|Default|GetIsJumping))
        (Class|EnemyAttackBPI|EnemyAttack(Message) OtherActor 1 (Variables|Default|GetBase))))))

(event EventBeginPlay
  (bind _location (CallFunction|GetBaseLocation))
  (bind _output_get (Variables|Default|SetBase _location))
  (Variables|Default|SetTarget _output_get)
  (Variables|Default|SetBaseOffset (- (Transformation|GetWorldLocation (Variables|Default|GetBaseLocation)) (Transformation|GetWorldLocation (Variables|Transformation|GetRootComponent))))
  (Variables|Default|SetBaseRelativeOffset (Variables|/Script/Engine.SceneComponent|GetRelativeLocation (Variables|Default|GetSpringEnemy_Bottom_DM))))

(event Collision|EventActorBeginOverlap
  (params (OtherActor :type Actor%20Object%20Reference)))

(event EventTick
  (params (DeltaSeconds :type Float%20%28single-precision%29))
  (Variables|Default|SetCurrentTime (+ DeltaSeconds (Variables|Default|GetCurrentTime)))
  (if (Variables|Default|GetIsDead)
    ;[1 1 1] 死んでるとき
    (if (> (Variables|Default|GetCurrentTime) 8.0)
      (Utilities|FlowControl|DoOnce false
        (:Completed
          (Actor|DestroyActor))))
    (elif (Variables|Default|GetIsJumping)
      (Variables|Default|SetCurrentTime (Math|Float|Min(Float) (Variables|Default|GetCurrentTime) (Variables|Default|GetBeatDuration)))
      (Transformation|SetActorLocation (+ (Math|Vector|Lerp(Vector) (Variables|Default|GetBase) (Variables|Default|GetTarget) (/ (Variables|Default|GetCurrentTime) (Variables|Default|GetBeatDuration))) (* (Variables|Default|GetUpVector) (* (Math|Trig|Sin(Degrees) (* (/ (Variables|Default|GetCurrentTime) (Variables|Default|GetBeatDuration)) 1.8e+02)) 3e+02))) true false)
      (Transformation|SetRelativeLocation (Variables|Default|GetSpringEnemy_Bottom_DM) (+ (Variables|Default|GetBaseRelativeOffset) (* (Variables|Default|GetSpringMoveVector) (Math|Curves|GetFloatValue (Variables|Default|GetSpringCurve) (/ (Variables|Default|GetCurrentTime) (Variables|Default|GetBeatDuration))))) false true))))

(event EventSetBPM
  (params (BPM :type Float%20%28single-precision%29) (Divide :type Float%20%28single-precision%29))
  ;[1 1 1] 拍の間隔の取得
  (bind _duration (CallFunction|GetBeatDuration BPM Divide))
  (Variables|Default|SetBeatDuration _duration)
  (Variables|Default|SetCurrentTime 0.0))

(event EventBeatFunction
  ;[1 1 1] BeatAction
  (if (not (Variables|Default|GetIsDead))
    (Class|BeatBPI|BeatFunction(Message) (AI|GetAIController self))
    (Variables|Default|SetCurrentTime 0.0)
    ;[1 1 1] 攻撃する
    (Utilities|FlowControl|DoOnce false) ; enters at Reset
  ))

(event EventPlayerAttack
  (bind _capsulecomponent (Variables|Collision|GetCapsuleComponent))
  (bind _returnvalue (Transformation|GetWorldLocation _capsulecomponent))
  ;[1 1 1] 攻撃を受けた
  (Utilities|FlowControl|DoOnce false
    (:Completed
      (Variables|Default|SetIsDead true)
      (Class|DestructibleComponent|ApplyRadiusDamage (Variables|Default|GetSpringEnemy_Top_DM) 1.0 _returnvalue 1e+02 3e+03 true)
      (Class|DestructibleComponent|ApplyRadiusDamage (Variables|Default|GetSpringEnemy_Bottom_DM) 1.0 _returnvalue 1e+02 3e+03 true)
      (Pawn|UnPossess (AI|GetAIController self))
      (Collision|SetCollisionEnabled (Variables|Collision|GetCapsuleComponent) "NoCollision"))))

(fn ConstructionScript)

(fn GetBaseLocation
  (return (Transformation|GetWorldLocation (Variables|Default|GetBaseLocation))))

(fn ExecuteJump
  (params (TargetLocation :type Vector))
  (Variables|Default|SetTarget (- TargetLocation (Variables|Default|GetBaseOffset)))
  (bind _location (CallFunction|GetBaseLocation))
  (Variables|Default|SetBase _location)
  (Variables|Default|SetIsJumping true)
  (Transformation|SetActorRotation (Math|Conversions|RotationFromXVector (Math|Vector|MakeVector (.x (- (Variables|Default|GetTarget) (Variables|Default|GetBase))) (.y (- (Variables|Default|GetTarget) (Variables|Default|GetBase))) 0.0)))
  (Physics|SetEnableGravity (Variables|Collision|GetCapsuleComponent) false))

(fn SetIdle
  (Variables|Default|SetIsJumping false)
  (Transformation|SetRelativeLocation (Variables|Default|GetSpringEnemy_Bottom_DM) (Variables|Default|GetBaseRelativeOffset) true false)
  (Physics|SetEnableGravity (Variables|Collision|GetCapsuleComponent) true))